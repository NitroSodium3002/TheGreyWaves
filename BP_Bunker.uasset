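; Bunker actor that periodically shuts its door on a "greywave" countdown and tracks whether the player is inside.
; A timeline event track pings the speaker and decrements the counter; at zero it resets the counter and rotates the door shut, reversing after a delay.
; A DoOnce limits the metallic slam to the first update of each door movement.
; Entry and leaving trigger boxes set the ContainingPlayer flag and print debug messages.
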(event OnComponentBeginOverlap(EntryBox)
  (params (OverlappedComponent :type Primitive%20Component%20Object%20Reference) (OtherActor :type Actor%20Object%20Reference) (OtherComp :type Primitive%20Component%20Object%20Reference) (OtherBodyIndex :type Integer) (bFromSweep :type Boolean) (SweepResult :type Hit%20Result%20Structure%20%28by%20ref%29))
  (Utilities|Casting|CastToBP_FirstPersonCharacter OtherActor)
  (Variables|Default|SetContainingPlayer true)
  (Development|PrintString "MAN INSIDE"))

(event OnComponentBeginOverlap(LeavingBox)
  (params (OverlappedComponent :type Primitive%20Component%20Object%20Reference) (OtherActor :type Actor%20Object%20Reference) (OtherComp :type Primitive%20Component%20Object%20Reference) (OtherBodyIndex :type Integer) (bFromSweep :type Boolean) (SweepResult :type Hit%20Result%20Structure%20%28by%20ref%29))
  (Utilities|Casting|CastToBP_FirstPersonCharacter OtherActor)
  (Variables|Default|SetContainingPlayer false)
  (Development|PrintString "NO MAN INSIDE"))

(event EventBeginPlay
  (Timeline|Count Play
    (:NewTrack_0
      (Audio|SpawnSoundAttached "/Engine/EngineSounds/1kSineTonePing.1kSineTonePing" (Variables|Default|GetSpeaker) "None" "0, 0, 0" "0, 0, 0" "KeepRelativeOffset" false 1.0 1.0 0.0 "/Game/UniversalAttenuator.UniversalAttenuator" 0)
      (bind _result (Math|Integer|DecrementInt (Variables|Default|GetGreywaveCounter))
        (:%20%20
          (if (== _result 0)
            (Variables|Default|SetGreywaveCounter 120)
            (Utilities|FlowControl|Sequence
              (:then_0
                (bind _newtrack_0 (Timeline|DoorShut Play)
                  (:Update
                    (Transformation|SetRelativeRotation (Variables|Default|GetScene) (Math|Rotator|MakeRotator 9e+02 _newtrack_0 9e+02) false false)
                    (Utilities|FlowControl|DoOnce false :!label _label
                      (:Completed
                        (Audio|SpawnSoundAttached "/Game/metallic_slam_jump_sfx.metallic_slam_jump_sfx" (Variables|Default|GetSpeaker) "None" "0, 0, 0" "0, 0, 0" "KeepRelativeOffset" false 1.0 1.0 0.0 "/Game/UniversalAttenuator.UniversalAttenuator" 0))))
                  (:Finished
                    (goto _label Reset))))
              (:then_1
                (Utilities|FlowControl|Delay 1e+01)
                (Timeline|DoorShut Reverse)))))))))

(event Collision|EventActorBeginOverlap
  (params (OtherActor :type Actor%20Object%20Reference)))

(event EventTick
  (params (DeltaSeconds :type Float%20%28single-precision%29)))

(fn ConstructionScript)