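; Escape helicopter actor that plays a one-shot startup and departure sequence when the player interacts with it.
; Interaction plays the startup sound and runs parallel timeline chains that rotate the two rotor pivots through successive spin stages, with timed delays leading to Takeoff.
; Takeoff rolls a third pivot, then animates the helicopter's location and pitch.
; An event on the flight timeline calls MysteryContact on the player character, and the actor destroys itself when flight ends.
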(event Custom|Takeoff
  (bind _newtrack_0 (Timeline|Timeline_8 Play)
    (:Update
      (Transformation|SetRelativeRotation (Variables|Default|GetScene2) (Math|Rotator|MakeRotator _newtrack_0 0.0 0.0) false false))
    (:Finished
      (Utilities|FlowControl|Sequence
        (:then_0
          (bind _newtrack_0_2 (Timeline|Timeline_9 Play)
            (:Update
              (Transformation|SetRelativeLocation (Variables|Default|Getlynx_helicopter) _newtrack_0_2 false false))
            (:Finished
              (Actor|DestroyActor))
            (:other
              (bind _asbp_first_person_character (Utilities|Casting|CastToBP_FirstPersonCharacter (Game|GetPlayerCharacter 0)))
              (Default|MysteryContact _asbp_first_person_character))))
        (:then_1
          (bind _newtrack_0_3 (Timeline|Timeline_10 PlayFromStart)
            (:Update
              (Transformation|SetRelativeRotation (Variables|Default|Getlynx_helicopter) (Math|Rotator|MakeRotator 1.8e+02 _newtrack_0_3 0.0) false false))))))))

(event EventBeginPlay)

(event Collision|EventActorBeginOverlap
  (params (OtherActor :type Actor%20Object%20Reference)))

(event EventTick
  (params (DeltaSeconds :type Float%20%28single-precision%29)))

(event EventFuncPlayerInteract
  (Utilities|FlowControl|DoOnce false
    (:Completed
      (Audio|SpawnSoundAttached "/Game/helicopter_startup_sfx.helicopter_startup_sfx" (Variables|Default|GetSpeaker) "None" "0, 0, 0" "0, 0, 0" "KeepRelativeOffset" false 1.0 1.0 0.0 "/Game/ChopperAttenuation.ChopperAttenuation" 0)
      (Utilities|FlowControl|Sequence
        (:then_0
          (bind _newtrack_0 (Timeline|SpinTop PlayFromStart)
            (:Update
              (Transformation|SetRelativeRotation (Variables|Default|GetScene) (Math|Rotator|MakeRotator 0.0 0.0 _newtrack_0) false false))
            (:Finished
              (bind _newtrack_0_2 (Timeline|Timeline PlayFromStart)
                (:Update
                  (Transformation|SetRelativeRotation (Variables|Default|GetScene) (Math|Rotator|MakeRotator 0.0 0.0 _newtrack_0_2) false false))
                (:Finished
                  (bind _newtrack_0_3 (Timeline|Timeline_1 PlayFromStart)
                    (:Update
                      (Transformation|SetRelativeRotation (Variables|Default|GetScene) (Math|Rotator|MakeRotator 0.0 0.0 _newtrack_0_3) false false))
                    (:Finished
                      (Utilities|FlowControl|Sequence
                        (:then_0
                          (bind _newtrack_0_4 (Timeline|Timeline_11 Play)
                            (:Update
                              (Transformation|SetRelativeRotation (Variables|Default|GetScene) (Math|Rotator|MakeRotator 0.0 0.0 _newtrack_0_4) false false))))
                        (:then_1
                          (Utilities|FlowControl|Delay 1e+01)
                          (Utilities|FlowControl|Sequence
                            (:then_0
                              (Timeline|Timeline_11 Stop))
                            (:then_1
                              (bind _newtrack_0_5 (Timeline|Timeline_2 PlayFromStart)
                                (:Update
                                  (Transformation|SetRelativeRotation (Variables|Default|GetScene) (Math|Rotator|MakeRotator 0.0 0.0 _newtrack_0_5) false false))))))))))))))
        (:then_1
          (bind _newtrack_0_6 (Timeline|Timeline_3 PlayFromStart)
            (:Update
              (Transformation|SetRelativeRotation (Variables|Default|GetScene1) (Math|Rotator|MakeRotator 0.0 _newtrack_0_6 0.0) false false))
            (:Finished
              (bind _newtrack_0_7 (Timeline|Timeline_4 PlayFromStart)
                (:Update
                  (Transformation|SetRelativeRotation (Variables|Default|GetScene1) (Math|Rotator|MakeRotator 0.0 _newtrack_0_7 0.0) false false))
                (:Finished
                  (bind _newtrack_0_8 (Timeline|Timeline_6 PlayFromStart)
                    (:Update
                      (Transformation|SetRelativeRotation (Variables|Default|GetScene1) (Math|Rotator|MakeRotator 0.0 _newtrack_0_8 0.0) false false))
                    (:Finished
                      (Utilities|FlowControl|Sequence
                        (:then_0
                          (bind _newtrack_0_9 (Timeline|Timeline_5 PlayFromStart)
                            (:Update
                              (Transformation|SetRelativeRotation (Variables|Default|GetScene1) (Math|Rotator|MakeRotator 0.0 _newtrack_0_9 0.0) false false))))
                        (:then_1
                          (Utilities|FlowControl|Delay 1e+01)
                          (Utilities|FlowControl|Sequence
                            (:then_0
                              (Timeline|Timeline_5 Stop))
                            (:then_1
                              (bind _newtrack_0_10 (Timeline|Timeline_7 PlayFromStart)
                                (:Update
                                  (Transformation|SetRelativeRotation (Variables|Default|GetScene1) (Math|Rotator|MakeRotator 0.0 _newtrack_0_10 0.0) false false))))
                            (:then_2
                              (Utilities|FlowControl|Delay 4e+01)
                              (CallFunction|Takeoff))))))))))))))))

(fn ConstructionScript)