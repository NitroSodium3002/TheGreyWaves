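; BP_EscapeSub is an escape submarine actor that surfaces on cue and ends the level successfully when the player interacts with it.
; On BeginPlay a timeline animates the sub mesh's pitch.
; The Emerge event waits, drives the actor's world Z from a second timeline, then plays an attenuated water splash when finished.
; FuncPlayerInteract opens the L_Success1 level.
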(event Custom|Emerge
  (bind _returnvalue (Transformation|GetActorLocation))
  (Utilities|FlowControl|Delay 1e+01)
  (bind _newtrack_0 (Timeline|Timeline PlayFromStart)
    (:Update
      (Transformation|SetActorLocation (Math|Vector|MakeVector (.x _returnvalue) (.y _returnvalue) _newtrack_0) false false))
    (:Finished
      (Audio|PlaySoundatLocation "/Game/water_splash_sfx.water_splash_sfx" (Transformation|GetActorLocation) "0, 0, 0" 1.0 1.0 0.0 "/Game/ChopperAttenuation.ChopperAttenuation" 0 0 0))))

(event EventBeginPlay
  (bind _g (Timeline|cvcgvbgfa\xc Play)
    (:Update
      (Transformation|SetRelativeRotation (Variables|Default|Getproteus_fantastic_voyage_1966) (Math|Rotator|MakeRotator 0.0 _g 0.0) false false))))

(event Collision|EventActorBeginOverlap
  (params (OtherActor :type Actor%20Object%20Reference)))

(event EventTick
  (params (DeltaSeconds :type Float%20%28single-precision%29)))

(event EventFuncPlayerInteract
  (Game|OpenLevel(byObjectReference) "/Game/L_Success1.L_Success1"))

(fn ConstructionScript)