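; BP_Greywave is a nanite "grey wave" hazard that sends the player to a death level on contact while active.
; PUNCHIT! activates it, revealing the Cube and sliding it along relative X with a timeline, then hiding it when finished.
; Overlapping a bunker that contains the player deactivates and hides the wave.
; Its attached, attenuated sound tracks the player's X and Z each tick while keeping its own Y.
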(event Custom|PUNCH%20IT!
  (bind _cube (Variables|Default|GetCube))
  (bind _relativelocation (Variables|/Script/Engine.SceneComponent|GetRelativeLocation _cube))
  (Development|PrintString "PUNCHING IT!")
  (Variables|Default|SetIsActive true)
  (Development|SetHiddeninGame (Variables|Default|GetCube) false false)
  (bind _newtrack_0 (Timeline|PUNCHING%20IT PlayFromStart)
    (:Update
      (Transformation|SetRelativeLocation _cube (Math|Vector|MakeVector _newtrack_0 (.y _relativelocation) (.z _relativelocation)) false false))
    (:Finished
      (Development|SetHiddeninGame (Variables|Default|GetCube) true false)
      (Development|PrintString "is now hidden"))))

(event EventBeginPlay
  (Audio|SpawnSoundAttached "/Game/grey_wave_nanite_sound.grey_wave_nanite_sound" (Variables|Default|GetAudio) "None" "0, 0, 0" "0, 0, 0" "KeepRelativeOffset" false 1.0 1.0 0.0 "/Game/GreywaveAttn.GreywaveAttn" 0))

(event EventTick
  (params (DeltaSeconds :type Float%20%28single-precision%29))
  (bind _audio (Variables|Default|GetAudio))
  (bind _asbp_first_person_character (Utilities|Casting|CastToBP_FirstPersonCharacter (Game|GetPlayerCharacter 0)))
  (Transformation|SetWorldLocation _audio (Math|Vector|MakeVector (.x (Transformation|GetActorLocation _asbp_first_person_character)) (.y (Transformation|GetWorldLocation _audio)) (.z (Transformation|GetActorLocation _asbp_first_person_character))) false false))

(event Collision|EventActorBeginOverlap
  (params (OtherActor :type Actor%20Object%20Reference))
  (Utilities|Casting|CastToBP_FirstPersonCharacter OtherActor
    (:then
      (if (Variables|Default|GetIsActive)
        (Game|OpenLevel(byObjectReference) "/Game/L_Death1.L_Death1")))
    (:CastFailed
      (bind _asbp_bunker (Utilities|Casting|CastToBP_Bunker OtherActor))
      (if (Variables|/Game/BP_Bunker.BP_Bunker_C|GetContainingPlayer _asbp_bunker)
        (Variables|Default|SetIsActive false)
        (Development|SetHiddeninGame (Variables|Default|GetCube) true false)
        (Development|PrintString "is now hidden")))))

(fn ConstructionScript)