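; BP_GreywaveCounter is an actor that counts down to each grey wave and launches it.
; On BeginPlay it plays the Count timeline, whose event track decrements GreywaveTime and sounds an alarm shortly before the wave.
; At zero it finds the BP_Greywave actor by class, calls PUNCHIT on it and resets the counter.
; A second timeline that also calls PUNCHIT is never run.
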(event EventBeginPlay
  (Timeline|Count Play
    (:NewTrack_0
      (Math|Integer|DecrementInt (Variables|Default|GetGreywaveTime)
        (:%20%20
          (if (== (Variables|Default|GetGreywaveTime) 20)
            (Audio|PlaySound2D "/Game/grey_wave_alarm_sound.grey_wave_alarm_sound" 1.0 1.0 0.0 0 0)
            (elif (== (Variables|Default|GetGreywaveTime) 0)
              (bind _returnvalue (Actor|GetActorOfClass "/Game/BP_Greywave.BP_Greywave_C"))
              (Default|PUNCHIT! _returnvalue)
              (Variables|Default|SetGreywaveTime 120))))))))

(event Collision|EventActorBeginOverlap
  (params (OtherActor :type Actor%20Object%20Reference)))

(event EventTick
  (params (DeltaSeconds :type Float%20%28single-precision%29)))

(fn ConstructionScript)